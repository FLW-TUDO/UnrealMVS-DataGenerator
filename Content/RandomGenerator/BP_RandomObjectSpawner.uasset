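; BP_RandomObjectSpawner is an actor that fills a volume with a freshly randomized scatter of objects every frame.
; On Tick it destroys all actors of the ObjectToSpawn class, then spawns SpawnCount new ones at random world positions and rotations, with unit scale.
; Each spawned actor's static mesh component receives a random mesh from MeshArray and a random slot-0 material from MaterialArray.
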(event EventBeginPlay)

(event Collision|EventActorBeginOverlap
  (params (OtherActor :type Actor%20Object%20Reference)))

(event EventTick
  (params (DeltaSeconds :type Float%20%28single-precision%29))
  (bind _materialarray (Variables|Default|GetMaterialArray))
  (bind _mesharray (Variables|Default|GetMeshArray))
  (bind _outactors (Actor|GetAllActorsOfClass (Variables|Default|GetObjectToSpawn)))
  (for _array_element _outactors
    (Actor|DestroyActor _array_element))
  (for _index (range 0 (- (Variables|Default|GetSpawnCount) 1))
    (bind _returnvalue (Game|SpawnActorfromClass (Variables|Default|GetObjectToSpawn) (Math|Transform|MakeTransform (Math|Vector|MakeVector (Math|Random|RandomFloatinRange -1e+03 -1e+04) (Math|Random|RandomFloatinRange -1e+04 1e+04) (Math|Random|RandomFloatinRange -1e+04 1e+04)) (Math|Rotator|MakeRotator (Math|Random|RandomFloatinRange 0.0 3.6e+02) (Math|Random|RandomFloatinRange 0.0 3.6e+02) (Math|Random|RandomFloatinRange 0.0 3.6e+02))) "Undefined" "MultiplyWithRoot" 0 0))
    (Components|StaticMesh|SetStaticMesh (Actor|GetComponentbyClass _returnvalue "/Script/Engine.StaticMeshComponent") (Utilities|Array|Get(acopy) _mesharray (Math|Random|RandomIntegerinRange 0 (- (Utilities|Array|Length _mesharray) 1))))
    (Rendering|Material|SetMaterial (Actor|GetComponentbyClass _returnvalue "/Script/Engine.StaticMeshComponent") 0 (Utilities|Array|Get(acopy) _materialarray (Math|Random|RandomIntegerinRange 0 (- (Utilities|Array|Length _materialarray) 1))))))

(fn ConstructionScript)